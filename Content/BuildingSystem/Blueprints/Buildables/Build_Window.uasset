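; Buildable window for the building system that players can open and close through the InteractwithBuilds event.
; BeginPlay caches both meshes' world rotations, and a Timeline then swings the two panels in opposite yaw directions from those defaults, playing forward to open and in reverse to close.
; An IsOpening flag blocks interaction while the animation runs, and ReturnBoxes is left empty.
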(event `self.ReceiveBeginPlay`
  (bind _defaultrotation (`self.DefaultRotation`))
  (`KismetArrayLibrary.Array_Set` _defaultrotation 0 (`SceneComponent.K2_GetComponentRotation` (`self.StaticMesh`)))
  (`KismetArrayLibrary.Array_Set` _defaultrotation 1 (`SceneComponent.K2_GetComponentRotation` (`self.StaticMesh1`))))

(event `/Game/BuildingSystem/Blueprints/BuildInterface.InteractWithBuilds`
  (bind (_output_roll _output_pitch _output_yaw) (`KismetMathLibrary.BreakRotator` (`|GetArrayItem` (`self.DefaultRotation`) 1)))
  (bind (_output_roll_2 _output_pitch_2 _output_yaw_2) (`KismetMathLibrary.BreakRotator` (`|GetArrayItem` (`self.DefaultRotation`))))
  (if (not (`self.IsOpening`))
    (if (not (`self.IsOpen`))
      (set `self.IsOpen` true)
      (bind (_direction _newtrack_0) (`Timeline|Timeline` :!via `PlayFromStart` :!label _label)
        (:`Update`
          (set `self.IsOpening` true)
          (`SceneComponent.K2_SetWorldRotation` (`self.StaticMesh`) (`KismetMathLibrary.MakeRotator` 0.0 0.0 (+ _newtrack_0 _output_yaw_2)) false false)
          (`SceneComponent.K2_SetWorldRotation` (`self.StaticMesh1`) (`KismetMathLibrary.MakeRotator` 0.0 0.0 (+ (* _newtrack_0 -1.0) _output_yaw)) false false))
        (:`Finished`
          (set `self.IsOpening` false)))
      (else
        (set `self.IsOpen` false)
        (goto _label :!via `ReverseFromEnd`)))))

(fn `ReturnBoxes`
  (returns (Boxes :type "Array of BoxComponent Object Reference"))
  (return))

(fn `UserConstructionScript`)