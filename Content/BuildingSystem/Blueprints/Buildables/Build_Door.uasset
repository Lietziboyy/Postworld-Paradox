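; Build_Door is a buildable door in the building system that swings open and closed when the player interacts with it.
; BeginPlay caches the mesh's starting world rotation, and InteractwithBuilds plays a timeline forward or in reverse to offset the yaw from that default.
; An IsOpening flag blocks new interactions while the timeline runs, and IsOpen picks the direction.
; ReturnBoxes is implemented empty.
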(event `self.ReceiveBeginPlay`
  (set `self.DefaultRotation` (`SceneComponent.K2_GetComponentRotation` (`self.StaticMeshComponent`))))

(event `/Game/BuildingSystem/Blueprints/BuildInterface.InteractWithBuilds`
  (bind (_defaultrotation_roll _defaultrotation_pitch _defaultrotation_yaw) (`KismetMathLibrary.BreakRotator` (`self.DefaultRotation`)))
  (if (not (`self.IsOpening`))
    (if (not (`self.IsOpen`))
      (set `self.IsOpen` true)
      (bind (_direction _newtrack_0) (`Timeline|Timeline` :!via `PlayFromStart` :!label _label)
        (:`Update`
          (set `self.IsOpening` true)
          (`SceneComponent.K2_SetWorldRotation` (`self.StaticMeshComponent`) (`KismetMathLibrary.MakeRotator` 0.0 0.0 (+ _newtrack_0 _defaultrotation_yaw)) false false))
        (:`Finished`
          (set `self.IsOpening` false)))
      (else
        (set `self.IsOpen` false)
        (goto _label :!via `ReverseFromEnd`)))))

(fn `ReturnBoxes`
  (returns (Boxes :type "Array of BoxComponent Object Reference"))
  (return))

(fn `UserConstructionScript`)