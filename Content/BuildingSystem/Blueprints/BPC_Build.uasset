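; Build-mode component for BP_ThirdPersonCharacter that previews and spawns buildables loaded from the DB_Buildables data table.
; A loop repeating every 0.1 seconds traces from the camera, moving a ghost mesh that snaps to snap boxes reported by the hit actor.
; GiveBuildColor tints the ghost green or red and writes that result to IsBuildMode, so a missed trace with a valid ghost ends build mode.
; SpawnBuild spawns the selected actor at the preview transform.
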(event `self.ReceiveBeginPlay`
  ;[0.05127 0.05127 0.05127] Feeding variables
  (bind _asbp_third_person_character (cast `/Game/ThirdPerson/Blueprints/BP_ThirdPersonCharacter` (`self.GetOwner`)))
  (set `self.PlayerReference` _asbp_third_person_character)
  (bind _outrownames (`DataTableFunctionLibrary.GetDataTableRowNames` "/Game/BuildingSystem/Blueprints/DB_Buildables.DB_Buildables"))
  (for _array_element _outrownames
    (bind _returnvalue (`|GetDataTableRow` "/Game/BuildingSystem/Blueprints/DB_Buildables.DB_Buildables" _array_element)
      (:`then`
        (`KismetArrayLibrary.Array_Add` (`self.Buildables`) _returnvalue)
        (bind _returnvalue_2 (`|AddComponentByClass` (`self.PlayerReference`) "/Script/Engine.StaticMeshComponent" false (`self.BuildTransform`)))
        (set `self.BuildGhost` _returnvalue_2)))))

(event `BuildDelay`
  (bind _buildghost (`self.BuildGhost`))
  ;[0.05127 0.05127 0.05127] Build Delay
  (if (`self.IsBuildMode`)
    (`KismetSystemLibrary.Delay` 0.1)
    (`self.BuildCycle`)
    (else
      (set `self.IsBuildMode` false :!label _label)
      (set `self.CanBuild` false)
      (`/Engine/EditorBlueprintResources/StandardMacros.IsValid` _buildghost
        (:`Is Valid`
          (`/Game/ThirdPerson/Blueprints/BP_ThirdPersonCharacter.DestroyComponent` (`self.PlayerReference`) _buildghost))))))

(event `StopBuildMode`
  ;[0.05127 0.05127 0.05127] Build Delay
  (goto _label))

(event `LaunchBuildMode`
  ;[0.05127 0.05127 0.05127] Launch Build Mode
  (if (`self.IsBuildMode`)
    (`self.StopBuildMode`)
    (else
      (set `self.IsBuildMode` true)
      (`self.BuildCycle`))))

(fn `BuildCycle`
  (bind _camera (`self.Camera`))
  (bind (_buildtransform_location _buildtransform_rotation _buildtransform_scale) (`KismetMathLibrary.BreakTransform` (`self.BuildTransform`)))
  (bind _buildghost (`self.BuildGhost`))
  (bind _returnvalue (`SceneComponent.K2_GetComponentLocation` _camera))
  (bind _returnvalue_2 (`SceneComponent.GetForwardVector` _camera))
  (bind (_output_mesh _output_tracechannel) (break `/Game/BuildingSystem/Blueprints/S_Buildables` (`|GetArrayItem` (`self.Buildables`) (`self.BuildID`))))
  (bind (_outhit _returnvalue_3) (`KismetSystemLibrary.LineTraceSingle` :`Start` (+ _returnvalue (* _returnvalue_2 350)) :`End` (+ _returnvalue (* _returnvalue_2 1000)) :`TraceChannel` _output_tracechannel :`DrawDebugType` "Persistent"))
  (if _returnvalue_3
    (bind (_bblockinghit _binitialoverlap _time _distance _location _impactpoint _normal _impactnormal _physmat _hitactor _hitcomponent _hitbonename _bonename _hititem _elementindex _faceindex _tracestart _traceend) (`GameplayStatics.BreakHitResult` _outhit))
    (set `self.BuildTransform` (`KismetMathLibrary.MakeTransform` _impactpoint _buildtransform_rotation _buildtransform_scale))
    (set `self.Hit Actor` _hitactor)
    (set `self.Hit Component` _hitcomponent)
    (`/Engine/EditorBlueprintResources/StandardMacros.IsValid` _buildghost
      (:`Is Valid`
        (bind (_found _transform) (`self.DetectBuildBoxes`))
        (if _found
          (set `self.BuildTransform` _transform))
        (`self.GiveBuildColor` true)
        (`self.BuildDelay`))
      (:`Is Not Valid`
        (`self.Spawn Build Ghost` :!label _label)
        (`self.BuildDelay` :!label _label_2)))
    (else
      (set `self.BuildTransform` (`KismetMathLibrary.MakeTransform` _traceend _buildtransform_rotation _buildtransform_scale))
      (`/Engine/EditorBlueprintResources/StandardMacros.IsValid` _buildghost
        (:`Is Valid`
          (`self.GiveBuildColor` false)
          (goto _label_2))
        (:`Is Not Valid`
          (goto _label))))))

(fn `ChangeMesh`
  (bind _output_mesh (break `/Game/BuildingSystem/Blueprints/S_Buildables` (`|GetArrayItem` (`self.Buildables`) (`self.BuildID`))))
  (`StaticMeshComponent.SetStaticMesh` (`self.BuildGhost`) _output_mesh))

(fn `DetectBuildBoxes`
  (returns (Found :type Boolean) (Transform :type "Transform Structure"))
  (locals (LocalFound :type Boolean))
  (bind _boxes (message `/Game/BuildingSystem/Blueprints/BuildInterface.ReturnBoxes` (`self.Hit Actor`)))
  (for _array_element _boxes
    (if (== _array_element (`self.Hit Component`))
      (set `local.LocalFound` true)
      (break)))
  (return (`local.LocalFound`) (`SceneComponent.K2_GetComponentToWorld` (`self.Hit Component`))))

(fn `GiveBuildColor`
  (params (IsGreen :type Boolean))
  (bind _buildghost (`self.BuildGhost`))
  (bind _output_get (set `self.IsBuildMode` IsGreen))
  (for _index (range (`PrimitiveComponent.GetNumMaterials` (`self.BuildGhost`)))
    (if _output_get
      (`PrimitiveComponent.SetMaterial` _buildghost _index "/Game/BuildingSystem/Assets/Colors/GreenColor.GreenColor")
      (else
        (`PrimitiveComponent.SetMaterial` _buildghost _index "/Game/BuildingSystem/Assets/Colors/RedColor.RedColor"))))
  (`SceneComponent.K2_SetWorldTransform` (`self.BuildGhost`) (`self.BuildTransform`) false false))

(fn `Spawn Build Ghost`
  (bind _output_mesh (break `/Game/BuildingSystem/Blueprints/S_Buildables` (`|GetArrayItem` (`self.Buildables`) (`self.BuildID`))))
  (bind _returnvalue (`|AddComponentByClass` (`self.PlayerReference`) "/Script/Engine.StaticMeshComponent" false (`self.BuildTransform`)))
  (bind _output_get (set `self.BuildGhost` _returnvalue))
  (`StaticMeshComponent.SetStaticMesh` _output_get _output_mesh)
  (`PrimitiveComponent.SetCollisionEnabled` (`self.BuildGhost`) "NoCollision"))

(fn `SpawnBuild`
  (bind (_output_mesh _output_tracechannel _output_actor) (break `/Game/BuildingSystem/Blueprints/S_Buildables` (`|GetArrayItem` (`self.Buildables`) (`self.BuildID`))))
  (bind _returnvalue (`|SpawnActorFromClass` _output_actor (`self.BuildTransform`) "Undefined" "MultiplyWithRoot" null null))
  (message `/Game/BuildingSystem/Blueprints/BuildInterface.SetMesh` _returnvalue _output_mesh))