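; Player stats component for the third-person character that tracks health, hunger, XP and level.
; BeginPlay waits a tick, caches the owning character and fills its HUD widget.
; Health and hunger functions update the HUD directly, cap gains at max, and report depletion on decreases.
; Reaching max XP resets XP and raises its threshold, but passes zero levels to IncreaseLevel; the XP bar refreshes only then.
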(event `self.ReceiveBeginPlay`
  (bind _hud_widget (`/Game/ThirdPerson/Blueprints/BP_ThirdPersonCharacter.HUD Widget` (`self.Player Character BP`)))
  (bind _hud_widget_2 (`/Game/ThirdPerson/Blueprints/BP_ThirdPersonCharacter.HUD Widget` (`self.Player Character BP`)))
  ;[0.05127 0.05127 0.05127] preloading the UI
  (`KismetSystemLibrary.DelayUntilNextTick`)
  (bind _asbp_third_person_character (cast `/Game/ThirdPerson/Blueprints/BP_ThirdPersonCharacter` (`self.GetOwner`)))
  (set `self.Player Character BP` _asbp_third_person_character)
  (`ProgressBar.SetPercent` (`/Game/UI/WB_HUD.Health_Bar` _hud_widget_2) (/ (`self.Current Health`) (`self.Max health`)))
  (`TextBlock.SetText` (`/Game/UI/WB_HUD.Health_Text` _hud_widget_2) (`KismetTextLibrary.Conv_StringToText` (`KismetStringLibrary.Concat_StrStr` (`KismetStringLibrary.Conv_DoubleToString` (`self.Current Health`)) "/" (`KismetStringLibrary.Conv_DoubleToString` (`self.Max health`)))))
  (`ProgressBar.SetPercent` (`/Game/UI/WB_HUD.Hunger_Bar` _hud_widget) (/ (`self.Current Hunger`) (`self.Max Hunger`)))
  (`TextBlock.SetText` (`/Game/UI/WB_HUD.Hunger_Text` _hud_widget) "")
  (`ProgressBar.SetPercent` (`/Game/UI/WB_HUD.XP_Bar` (`/Game/ThirdPerson/Blueprints/BP_ThirdPersonCharacter.HUD Widget` (`self.Player Character BP`))) (/ (`self.XP`) (`self.Max XP`)))
  (`TextBlock.SetText` (`/Game/UI/WB_HUD.XP_Text` (`/Game/ThirdPerson/Blueprints/BP_ThirdPersonCharacter.HUD Widget` (`self.Player Character BP`))) (`|FormatText` "{Current XP} / {Max Xp}" (`self.XP`) (`self.Max XP`)))
  (`TextBlock.SetText` (`/Game/UI/WB_HUD.Level_Text` (`/Game/ThirdPerson/Blueprints/BP_ThirdPersonCharacter.HUD Widget` (`self.Player Character BP`))) (`KismetTextLibrary.Conv_IntToText` (`self.Level`))))

(fn `Decrease Health`
  (params (Damage :type "Float (double-precision)"))
  (returns (`IsPlayerDead?` :type Boolean))
  (bind _hud_widget (`/Game/ThirdPerson/Blueprints/BP_ThirdPersonCharacter.HUD Widget` (`self.Player Character BP`)))
  (if (not (<= (`self.Current Health`) 0.0))
    (bind _output_get (set `self.Current Health` (- (`self.Current Health`) Damage)))
    (`ProgressBar.SetPercent` (`/Game/UI/WB_HUD.Health_Bar` _hud_widget) (/ _output_get (`self.Max health`)))
    (`TextBlock.SetText` (`/Game/UI/WB_HUD.Health_Text` _hud_widget) (`KismetTextLibrary.Conv_StringToText` (`KismetStringLibrary.Concat_StrStr` (`KismetStringLibrary.Conv_DoubleToString` (`self.Current Health`)) "/" (`KismetStringLibrary.Conv_DoubleToString` (`self.Max health`)))))
    (if (<= (`self.Current Health`) 0.0)
      _
      (else
        (return false))))
  (return true))

(fn `Decrease Hunger`
  (params (`Hunger removed` :type "Float (double-precision)"))
  (returns (`No Hunger Left` :type Boolean))
  (bind _hud_widget (`/Game/ThirdPerson/Blueprints/BP_ThirdPersonCharacter.HUD Widget` (`self.Player Character BP`)))
  (if (not (<= (`self.Current Hunger`) 0.0))
    (set `self.Current Hunger` (- (`self.Current Hunger`) `Hunger removed`))
    (`ProgressBar.SetPercent` (`/Game/UI/WB_HUD.Hunger_Bar` _hud_widget) (/ (`self.Current Hunger`) (`self.Max Hunger`)))
    (`TextBlock.SetText` (`/Game/UI/WB_HUD.Hunger_Text` _hud_widget) (`KismetTextLibrary.Conv_StringToText` (`KismetStringLibrary.Concat_StrStr` (`KismetStringLibrary.Conv_DoubleToString` (`self.Current Hunger`)) "/" (`KismetStringLibrary.Conv_DoubleToString` (`self.Max Hunger`)))))
    (if (<= (`self.Current Hunger`) 0.0)
      _
      (else
        (return false))))
  (return true))

(fn `Increase Health`
  (params (`Added Health` :type "Float (double-precision)"))
  (bind _hud_widget (`/Game/ThirdPerson/Blueprints/BP_ThirdPersonCharacter.HUD Widget` (`self.Player Character BP`)))
  (set `self.Current Health` (+ (`self.Current Health`) `Added Health`))
  (if (> (`self.Current Health`) (`self.Max health`))
    (set `self.Current Health` (`self.Max health`)))
  (`ProgressBar.SetPercent` (`/Game/UI/WB_HUD.Health_Bar` _hud_widget) (/ (`self.Current Health`) (`self.Max health`)))
  (`TextBlock.SetText` (`/Game/UI/WB_HUD.Health_Text` _hud_widget) (`KismetTextLibrary.Conv_StringToText` (`KismetStringLibrary.Concat_StrStr` (`KismetStringLibrary.Conv_DoubleToString` (`self.Current Health`)) "/" (`KismetStringLibrary.Conv_DoubleToString` (`self.Max health`))))))

(fn `Increase Hunger`
  (params (`Added Hunger` :type "Float (double-precision)"))
  (bind _hud_widget (`/Game/ThirdPerson/Blueprints/BP_ThirdPersonCharacter.HUD Widget` (`self.Player Character BP`)))
  (set `self.Current Hunger` (+ `Added Hunger` (`self.Current Hunger`)))
  (if (> (`self.Current Hunger`) (`self.Max Hunger`))
    (set `self.Current Hunger` (`self.Max Hunger`)))
  (`ProgressBar.SetPercent` (`/Game/UI/WB_HUD.Hunger_Bar` _hud_widget) (/ (`self.Current Hunger`) (`self.Max Hunger`)))
  (`TextBlock.SetText` (`/Game/UI/WB_HUD.Hunger_Text` _hud_widget) (`KismetTextLibrary.Conv_StringToText` (`KismetStringLibrary.Concat_StrStr` (`KismetStringLibrary.Conv_DoubleToString` (`self.Current Hunger`)) "/" (`KismetStringLibrary.Conv_DoubleToString` (`self.Max Hunger`))))))

(fn `Increase Level`
  (params (`Added Level` :type Integer))
  (set `self.Level` (+ (`self.Level`) `Added Level`))
  (set `self.Max XP` (+ (`self.Max XP`) 150.0))
  (set `self.XP` 0.0)
  (`TextBlock.SetText` (`/Game/UI/WB_HUD.Level_Text` (`/Game/ThirdPerson/Blueprints/BP_ThirdPersonCharacter.HUD Widget` (`self.Player Character BP`))) (`KismetTextLibrary.Conv_IntToText` (`self.Level`))))

(fn `Increase Max Health`
  (params (`Health Increase` :type "Float (double-precision)"))
  (bind _hud_widget (`/Game/ThirdPerson/Blueprints/BP_ThirdPersonCharacter.HUD Widget` (`self.Player Character BP`)))
  (set `self.Max health` (+ (`self.Max health`) `Health Increase`))
  (`ProgressBar.SetPercent` (`/Game/UI/WB_HUD.Health_Bar` _hud_widget) (/ (`self.Current Health`) (`self.Max health`)))
  (`TextBlock.SetText` (`/Game/UI/WB_HUD.Health_Text` _hud_widget) (`KismetTextLibrary.Conv_StringToText` (`KismetStringLibrary.Concat_StrStr` (`KismetStringLibrary.Conv_DoubleToString` (`self.Current Health`)) "/" (`KismetStringLibrary.Conv_DoubleToString` (`self.Max health`))))))

(fn `Increase Max Hunger`
  (params (`Added Hunger` :type "Float (double-precision)"))
  (bind _hud_widget (`/Game/ThirdPerson/Blueprints/BP_ThirdPersonCharacter.HUD Widget` (`self.Player Character BP`)))
  (set `self.Max Hunger` (+ (`self.Max Hunger`) `Added Hunger`))
  (`ProgressBar.SetPercent` (`/Game/UI/WB_HUD.Hunger_Bar` _hud_widget) (/ (`self.Current Hunger`) (`self.Max Hunger`)))
  (`TextBlock.SetText` (`/Game/UI/WB_HUD.Hunger_Text` _hud_widget) (`KismetTextLibrary.Conv_StringToText` (`KismetStringLibrary.Concat_StrStr` (`KismetStringLibrary.Conv_DoubleToString` (`self.Current Hunger`)) "/" (`KismetStringLibrary.Conv_DoubleToString` (`self.Max Hunger`))))))

(fn `Increase XP`
  (params (`Added XP` :type "Float (double-precision)"))
  (set `self.XP` (+ `Added XP` (`self.XP`)))
  (if (>= (`self.XP`) (`self.Max XP`))
    (`self.Increase Level` 0)
    (`ProgressBar.SetPercent` (`/Game/UI/WB_HUD.XP_Bar` (`/Game/ThirdPerson/Blueprints/BP_ThirdPersonCharacter.HUD Widget` (`self.Player Character BP`))) (/ (`self.XP`) (`self.Max XP`)))
    (`TextBlock.SetText` (`/Game/UI/WB_HUD.XP_Text` (`/Game/ThirdPerson/Blueprints/BP_ThirdPersonCharacter.HUD Widget` (`self.Player Character BP`))) (`|FormatText` "{Current XP} / {Max Xp}" (`self.XP`) (`self.Max XP`)))))