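; Attack system Blueprint, apparently a component, for a montage-based sword combo triggered by the IA_Attack input when CanAttack is set.
; SwordAttack buffers input during an attack in SaveAttack, which SwordAttackCombo consumes to re-enter the AttackIndex switch; StopCombo resets the state.
; Attack1 plays its montage after a short delay behind a DoOnce and advances the index.
; The switch has no connected cases, and nothing here calls Attack1 or sets IsAttacking true.
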(event `Attack 1`
  ;[0.05127 0.05127 0.05127] Attack 1
  (`/Engine/EditorBlueprintResources/StandardMacros.DoOnce` false :!label _label
    (:`Completed`
      (`KismetSystemLibrary.Delay` 0.1)
      (`|PlayMontage` null "/Game/Characters/RPGCharacter/Animations/SwordAttacks/Attack1_Montage.Attack1_Montage"
        (:`then`
          (set `self.AttackIndex` 1)
          (goto _label :!via `Reset`))))))

(event `EnhancedInput|/Game/ThirdPerson/Input/Actions/IA_Attack`
  (params (ActionValue :type Boolean) (ElapsedSeconds :type "Float (double-precision)") (TriggeredSeconds :type "Float (double-precision)") (InputAction :type "InputAction Object Reference" :default "/Game/ThirdPerson/Input/Actions/IA_Attack.IA_Attack"))
  ;[0.05127 0.05127 0.05127] Attack Input
  (:`Started`
    (if (`self.canAttack?`)
      (`self.SwordAttack`))))

(event `SwordAttack`
  ;[0.05127 0.05127 0.05127] Sword Attack
  (if (`self.isAttacking?`)
    (set `self.saveAttack?` true)
    (else
      (set `self.saveAttack?` false)
      (switch `int` (`self.AttackIndex`) :!label _label_2))))

(event `SwordAttackCombo`
  ;[0.05127 0.05127 0.05127] Combo Continue
  (if (`self.saveAttack?`)
    (set `self.saveAttack?` false)
    (goto _label_2)))

(event `StopCombo`
  ;[0.05127 0.05127 0.05127] Stop Combo / Attack
  (set `self.isAttacking?` false)
  (set `self.AttackIndex` 0))