(event `self.ReceiveBeginPlay`
  (bind _asbp_third_person_character (cast `/Game/ThirdPerson/Blueprints/BP_ThirdPersonCharacter` (`Actor.GetOwner` (stale _output_get))))
  (bind _output_get (set `self.Player BP` _asbp_third_person_character))
  (set `self.Camera` (`/Game/ThirdPerson/Blueprints/BP_ThirdPersonCharacter.FollowCamera` _asbp_third_person_character)))

(event `Preview Loop`
  (bind (_returnvalue_location _returnvalue_rotation) (`KismetMathLibrary.BreakTransform` (`SceneComponent.K2_GetComponentToWorld`)))
  (bind (_outhit _returnvalue) (`KismetSystemLibrary.LineTraceSingle` :`Start` _returnvalue_location :`End` (+ _returnvalue_location (* (`KismetMathLibrary.GetForwardVector` _returnvalue_rotation) 70.0)) :`TraceChannel` "TraceTypeQuery1" :`DrawDebugType` "ForDuration"))
  (if _returnvalue
    (`|ExecutionSequence`
      (:`then_0`
        (`/Engine/EditorBlueprintResources/StandardMacros.DoOnce` false
          (:`Completed`
            (bind _returnvalue_2 (`|AddComponentByClass` (`self.Player BP`) "/Script/Engine.StaticMeshComponent" false (`self.Build Preview Transform`)))
            (set `self.Preview Mesh` _returnvalue_2))))
      (:`then_1`
        (bind _output_get (set `self.Build Preview Transform` (`KismetMathLibrary.MakeTransform` (`.Location` (`GameplayStatics.BreakHitResult` _outhit)))))
        (`SceneComponent.K2_SetWorldTransform` (`self.Preview Mesh`) _output_get false false)))))

(event `self.ReceiveTick`
  (params (DeltaSeconds :type "Float (single-precision)"))
  (if (`self.inBuildMode`)
    (`self.Preview Loop`)))

(event `EnhancedInput|/Game/ThirdPerson/Input/Actions/IA_Debug`
  (params (ActionValue :type Boolean) (ElapsedSeconds :type "Float (double-precision)") (TriggeredSeconds :type "Float (double-precision)") (InputAction :type "InputAction Object Reference" :default "/Game/ThirdPerson/Input/Actions/IA_Debug.IA_Debug"))
  (:`Started`
    (`/Engine/EditorBlueprintResources/StandardMacros.FlipFlop`
      (:`A`
        (set `self.inBuildMode` true))
      (:`B`
        (set `self.inBuildMode` false)))))